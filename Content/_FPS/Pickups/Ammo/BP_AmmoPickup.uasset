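; BP_AmmoPickup is a respawning pickup that adds reserve ammo of a set weapon type to an FPSCharacter that overlaps it.
; On overlap it hides the weapon mesh, plays sound and Niagara effects, switches collision to an inactive profile and sends the character an ammo message.
; A timer then restores collision and visibility, and Tick spins the mesh while the pickup is active.
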(event Custom|OnBeginOverlap
  (params (OverlappedComponent :type Primitive%20Component%20Object%20Reference) (OtherActor :type Actor%20Object%20Reference) (OtherComp :type Primitive%20Component%20Object%20Reference) (OtherBodyIndex :type Integer) (bFromSweep :type Boolean) (SweepResult :type Hit%20Result%20Structure%20%28by%20ref%29))
  (if (Variables|Default|GetIsActive)
    (bind _asfpscharacter (Utilities|Casting|CastToFPSCharacter OtherActor))
    (Variables|Default|SetOverlapedCharacter _asfpscharacter)
    (Utilities|FlowControl|Sequence
      (:then_0
        (Rendering|SetVisibility (Variables|Default|GetWeapon) false false)
        (Audio|PlaySoundatLocation (Variables|Default|GetPickupSound) (Transformation|GetActorLocation) "0, 0, 0" 1.0 1.0 0.0 0 0 0 0)
        (Niagara|SpawnSystematLocation (Variables|Default|GetParticleSystem) (+ (Transformation|GetActorLocation) "0.000000,0.000000,50.000000")))
      (:then_1
        (Collision|SetCollisionProfileName (Variables|Default|GetCollision) (Variables|Default|GetInactiveCollisionProfile) true :!class /Script/Engine.PrimitiveComponent)
        (Variables|Default|SetIsActive false)
        (Class|PlayerInterface|AddAmmoReserves(Message) (Variables|Default|GetOverlapedCharacter) (Variables|Default|GetWeaponType) (Variables|Default|GetAmount))
        (bind _returnvalue (Utilities|Time|SetTimerbyEvent (delegate Custom|OnRespawn) (Variables|Default|GetRespawnInterval)))
        (Variables|Default|SetRespawnTimer _returnvalue)))))

(event Custom|OnRespawn
  (Variables|Default|SetIsActive true)
  (Collision|SetCollisionProfileName (Variables|Default|GetCollision) (Variables|Default|GetActiveCollisionProfile) true :!class /Script/Engine.PrimitiveComponent)
  (Rendering|SetVisibility (Variables|Default|GetWeapon) true false))

(event EventBeginPlay
  (Collision|BindEventtoOnComponentBeginOverlap (Variables|Default|GetCollision) (delegate Custom|OnBeginOverlap)))

(event EventTick
  (params (DeltaSeconds :type Float%20%28single-precision%29))
  (if (Variables|Default|GetIsActive)
    (Transformation|AddLocalRotation (Variables|Default|GetWeapon) (Math|Rotator|MakeRotator 0.0 0.0 (* 6e+01 (Utilities|Time|GetWorldDeltaSeconds))) false false)))

(fn ConstructionScript)