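; Base FPS weapon Blueprint that plays cosmetic firing and dry-fire feedback.
; FireEffects skips dedicated servers, picks the first- or third-person mesh, caches impact data and muzzle location, then plays the fire sound and montage.
; It lazily spawns helper actors for muzzle/shell/tracer, impacts and decals, attaches them to the mesh, and feeds them the cached data on each shot.
; DryFireEffects only plays the dry-fire sound.
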(event EventDryFireEffects
  ;[0.15 0.15 0.15 0.5] Weapon Shooting Animation and Sound
  (Audio|PlaySoundatLocation (Variables|FPS|Weapon|Effects|GetWeaponDryFireSound) (Transformation|GetActorLocation) "0, 0, 0" 1.0 1.0 0.0 0 0 0 0))

(event EventFireEffects
  (params (ImpactPoint :type Vector%20%28by%20ref%29 :default "0, 0, 0") (ImpactNormal :type Vector%20%28by%20ref%29 :default "0, 0, 0") (ImpactSurfaceType :type EPhysicalSurface%20Enum :default "SurfaceType_Default") (bIsFirstPerson :type Boolean))
  (Variables|Default|SetIsFirstPerson bIsFirstPerson)
  (if (not (Networking|IsDedicatedServer))
    ;[0.15 0.15 0.15 0.5] Cache Effect Property Data
    (Variables|Default|SetImpactPoints (Utilities|Array|MakeArray ImpactPoint))
    (Variables|Default|SetImpactNormals (Utilities|Array|MakeArray ImpactNormal))
    (Variables|Default|SetImpactSurfaceTypes (Utilities|Array|MakeArray ImpactSurfaceType))
    (Utilities|FlowControl|Sequence
      (:then_0
        ;[0.15 0.15 0.15 0.5] Cache Skeletal Mesh
        (if (Variables|Default|GetIsFirstPerson)
          (Variables|Default|SetSkeletalMesh (Variables|Default|GetFirstPersonMesh))
          (else
            (Variables|Default|SetSkeletalMesh (Variables|Default|GetThirdPersonMesh)))))
      (:then_1
        ;[0.15 0.15 0.15 0.5] Cache Muzzle Position
        (Variables|Default|SetMuzlePosition (Transformation|GetSocketLocation (Variables|Default|GetSkeletalMesh) (Variables|Default|GetMuzzleSocketName))))
      (:then_2
        (Utilities|IsValid (Variables|Default|GetWeaponFire)
          (:Is%20Valid
            _)
          (:Is%20Not%20Valid
            (|SpawnAndSetupWeaponFire)))
        (|HandleWeaponFire))
      (:then_3
        (Utilities|IsValid (Variables|Default|GetWeaponImpacts)
          (:Is%20Valid
            _)
          (:Is%20Not%20Valid
            (|SpawnAndSetupWeaponInpacts)))
        (|HandleWeaponImpacts))
      (:then_4
        (Utilities|IsValid (Variables|Default|GetWeaponDecals)
          (:Is%20Valid
            _)
          (:Is%20Not%20Valid
            (|SpawnAndSetupWeaponDecals)))
        (|HandleWeaponDecals))
      (:then_5
        ;[0.15 0.15 0.15 0.5] Weapon Shooting Animation and Sound
        (Audio|PlaySoundatLocation (Variables|FPS|Weapon|Effects|GetWeaponFireSound) (Transformation|GetActorLocation) "0, 0, 0" 1.0 1.0 0.0 0 0 0 0)
        (Animation|Montage|PlayMontage (Variables|Default|GetSkeletalMesh) (Variables|FPS|Weapon|Animations|GetWeaponFireMontage))))))

(fn ConstructionScript)